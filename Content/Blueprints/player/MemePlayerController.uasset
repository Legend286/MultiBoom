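; Player controller that handles the pause menu, health HUD, player chat and image sprays.
; The health HUD drives a dynamic material with an eight-step index and a red-to-green colour.
; T multicasts the pause menu's URL, downloading the image unless it matches the last one, then projecting it as an aspect-scaled decal via camera trace.
; Chat messages go through the game mode's player list to each pause-menu chat window.
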(event Custom|CreateHUD%20on%20CLIENT
  (bind _returnvalue (UserInterface|CreateWidget "/Game/HUD/healthDisplay.healthDisplay_C" self))
  (bind _output_get (Variables|Default|SetHealth%20Widget _returnvalue))
  (bind _ashealth_display (Utilities|Casting|CastTohealthDisplay _output_get))
  (bind _returnvalue_2 (Appearance|GetDynamicMaterial (Variables|/Game/HUD/healthDisplay.healthDisplay_C|GetImage_18 _ashealth_display) :!class /Script/UMG.Image))
  (Variables|Default|Sethealth_dynamat _returnvalue_2)
  (UserInterface|Viewport|AddtoViewport _ashealth_display 0))

(event Custom|UPDATE%20HUD%20on%20CLIENT
  (params (Character :type %20Object%20Reference))
  (bind _health_dynamat (Variables|Default|Gethealth_dynamat))
  (bind _health (Variables|Default|Gethealth Character))
  (bind _maxhealth (Variables|Default|GetmaxHealth Character))
  (bind _returnvalue (Math|Conversions|ToFloat(Integer) _maxhealth))
  (bind _returnvalue_2 (Math|Conversions|ToFloat(Integer) _health))
  (bind _returnvalue_3 (- _returnvalue _returnvalue_2))
  (bind _returnvalue_4 (/ _returnvalue 8.0))
  (bind _returnvalue_5 (- _returnvalue _returnvalue_3))
  (bind _returnvalue_6 (/ _returnvalue_5 _returnvalue_4))
  (bind _returnvalue_7 (Math|Float|Ceil _returnvalue_6))
  (bind _returnvalue_8 (Math|Conversions|ToFloat(Integer) _returnvalue_7))
  (Development|PrintString "HUD UPDATE")
  (Development|PrintString (Utilities|String|ToString(Float) _returnvalue_8) true true "(R=0.000000,G=0.660000,B=1.000000,A=1.000000)" 0.0)
  (Rendering|Material|SetScalarParameterValue _health_dynamat "index" _returnvalue_8 :!class /Script/Engine.MaterialInstanceDynamic)
  (Rendering|Material|SetVectorParameterValue _health_dynamat "colour" (Class|KismetMathLibrary|HSVtoRGB (Math|Float|Lerp 0.0 1.2e+02 (/ _returnvalue_2 _returnvalue)) 1.0 1.0 1.0) :!class /Script/Engine.MaterialInstanceDynamic))

(event Custom|GetChatMessage
  (params (TextToSend :type Text))
  ;[1 1 1] Incoming chat message process on server
  (Variables|Default|SetSender%20Text TextToSend)
  (Variables|Default|SetSender%20Name (.Name (Utilities|Struct|Breakplayerinfo (Variables|Default|Getplayerinfo))))
  (bind _asdefault_mode (Utilities|Casting|CastTo (Game|GetGameMode)))
  (CallFunction|GetAllPlayers _asdefault_mode)
  (for _array_element (Variables|Default|Getplayers _asdefault_mode)
    (bind _output_get (Variables|Default|SetTimestamp (Math|DateTime|Now)))
    (CallFunction|UpdateChat _array_element (Variables|Default|GetSender%20Name) (Variables|Default|GetSender%20Text) _output_get)))

(event Custom|UpdateChat
  (params (Sender :type Text) (Message :type Text) (Timestamp :type Date%20Time%20Structure))
  (bind _chat (Default|GetChatWindow (Variables|Default|GetPaused%20Widget)))
  (Default|UpdateChat _chat Sender Message Timestamp))

(event Custom|spray_server
  (params (url :type String) (rotation :type Rotator))
  ;[1 1 1] Spray
  (CallFunction|SprayMulticast self url rotation))

(event Custom|spray_multicast
  (params (url :type String) (rotation :type Rotator))
  ;[1 1 1] Spray
  (Variables|Default|Setrotation%20camera rotation)
  (if (Utilities|Enum|Equal(Enum) url (Variables|Default|GetlastURL))
    _
    (else
      (Variables|Default|SetlastURL url)
      (bind _texture (|DownloadImage url)
        (:OnSuccess
          (Variables|Default|Setaspect_ratio (/ (Math|Conversions|ToFloat(Integer) (Class|Texture2D|BlueprintGetSizeX _texture)) (Math|Conversions|ToFloat(Integer) (Class|Texture2D|BlueprintGetSizeY _texture))))))))
  (bind _asmeme_player_character (Utilities|Casting|CastTo (Pawn|GetControlledPawn)))
  (bind _returnvalue (Rendering|Material|CreateDynamicMaterialInstance "/Game/Materials/Spray_Material.Spray_Material" "None" :!class /Script/Engine.KismetMaterialLibrary))
  (bind _output_get (Variables|Default|Setspray_mat _returnvalue))
  (Rendering|Material|SetTextureParameterValue _output_get "TextureParam" _texture)
  (bind _outhit (Collision|LineTraceByChannel (Transformation|GetWorldLocation (Variables|Default|Getfps_cam _asmeme_player_character)) (+ (Transformation|GetWorldLocation (Variables|Default|Getfps_cam _asmeme_player_character)) (* (Math|Vector|GetForwardVector (Variables|Default|Getrotation%20camera _asmeme_player_character)) 7e+02)) "TraceTypeQuery1" false 0 "None"))
  (Rendering|Decal|SpawnDecalatLocation 0 (Math|Vector|MakeVector 0.1 1.5e+02 (* -1.5e+02 (Variables|Default|Getaspect_ratio))) (.Location (Collision|BreakHitResult _outhit)) (Math|Rotator|MakeRotator (+ (.Roll (Math|Rotator|BreakRotator (Math|Conversions|RotationFromXVector (.ImpactNormal (Collision|BreakHitResult _outhit))))) 9e+01) (.Pitch (Math|Rotator|BreakRotator (Math|Conversions|RotationFromXVector (.ImpactNormal (Collision|BreakHitResult _outhit))))) (.Yaw (Math|Rotator|BreakRotator (Math|Conversions|RotationFromXVector (.ImpactNormal (Collision|BreakHitResult _outhit)))))) 0.0))

(event EventBeginPlay
  (Utilities|IsValid (Variables|Default|GetHealth%20Widget)
    (:Is%20Valid
      (CallFunction|UPDATEHUDonCLIENT))
    (:Is%20Not%20Valid
      (CallFunction|CreateHUDonCLIENT))))

(event Input|ActionEvents|InputActionMenu
  (params (Key :type Key%20Structure))
  (bind _self self)
  ;[1 1 1] Pause
  (:Pressed
    (bind _output_get (Variables|Default|SetPaused (not (Variables|Default|GetPaused))))
    (if _output_get
      (if (Utilities|IsValid (Variables|Default|GetPaused%20Widget))
        _
        (else
          (bind _returnvalue (UserInterface|CreateWidget "/Game/Menu/Pause.Pause_C" _self))
          (bind _output_get_2 (Variables|Default|SetPaused%20Widget _returnvalue))))
      (UserInterface|Viewport|AddtoViewport _output_get_2 5)
      (Input|SetInputModeGameandUI _self (Variables|Default|GetPaused%20Widget) false true)
      (Variables|/Script/Engine.PlayerController|SetbShowMouseCursor _self true)
      (else
        (Widget|RemovefromParent (Variables|Default|GetPaused%20Widget))
        (Input|SetInputModeGameOnly _self)
        (Variables|/Script/Engine.PlayerController|SetbShowMouseCursor _self false)
        (Class|WidgetBlueprintLibrary|SetFocustoGameViewport)))))

(event Input|KeyboardEvents|T
  (params (Key :type Key%20Structure))
  ;[1 1 1] Spray
  (:Pressed
    (bind _asmeme_player_character (Utilities|Casting|CastToMemePlayerCharacter (Pawn|GetControlledPawn)))
    (CallFunction|SprayMulticast (Utilities|String|ToString(Text) (Class|EditableTextBox|GetText (Variables|/Game/Menu/Pause.Pause_C|GetEditableTextBox_18 (Variables|Default|GetPaused%20Widget)))) (Transformation|GetWorldRotation (Variables|/Script/Engine.Character|GetCapsuleComponent _asmeme_player_character)))))

(fn ConstructionScript)